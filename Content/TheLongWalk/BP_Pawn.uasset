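; BP_Pawn is an on-rails player pawn that advances along a referenced spline path while IsWalking is true and carries a flashlight.
; Tick moves it by speed, plays distance-based footsteps, triggers camera shake and smoothly rotates toward spline rotation plus a target offset.
; BeginPlay adds the WDG_Avancer widget and shows the cursor.
; F press and release share a FlipFlop toggling the spotlight; Tick reduces a battery value while lit.
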(event `self.ReceiveBeginPlay`
  ; Comment
  (`|ExecutionSequence`
    (:`then_0`
      (if (`self.is walking`) :!label _label
        (`|ExecutionSequence`
          (:`then_0`
            (`/Engine/EditorBlueprintResources/StandardMacros.DoOnce` false :!label _label_2
              (:`Completed`
                (`LegacyCameraShake.StartLegacyCameraShake` (`GameplayStatics.GetPlayerCameraManager` 0) "/Game/TheLongWalk/CamSHake.CamSHake_C" 5.0))))
          (:`then_1`
            (set `self.distanceactuelle` (+ (* (`self.vitesse`) (`GameplayStatics.GetWorldDeltaSeconds`)) (`self.distanceactuelle`)))
            (`|ExecutionSequence`
              (:`then_0`
                (`self.K2_SetActorLocation` (`SplineComponent.GetLocationAtDistanceAlongSpline` (`/Game/TheLongWalk/BP_Chemin.CHemin` (`self.refchemin`)) (`self.distanceactuelle`) "World"))
                (set `self.distancedepuisdernierpas` (+ (* (`self.vitesse`) (`GameplayStatics.GetWorldDeltaSeconds`)) (`self.distancedepuisdernierpas`)))
                (if (> (`self.distancedepuisdernierpas`) 100.0)
                  (`GameplayStatics.PlaySound2D` "/Game/FootstepsMiniPack/SoundCue/Undergrowth_Mono_03_Cue.Undergrowth_Mono_03_Cue" 1.0 1.0 0.0 null null)
                  (set `self.distancedepuisdernierpas` 0.0)))
              (:`then_1`
                (`self.K2_SetActorRotation` (`KismetMathLibrary.RInterpTo` (`self.K2_GetActorRotation`) (`KismetMathLibrary.ComposeRotators` (`SplineComponent.GetRotationAtDistanceAlongSpline` (`/Game/TheLongWalk/BP_Chemin.CHemin` (`self.refchemin`)) (`self.distanceactuelle`) "World") (`self.TARGET ROTATION`)) (`GameplayStatics.GetWorldDeltaSeconds`) 5.0))))))
        (else
          (`|ExecutionSequence`
            (:`then_0`
              (goto _label_2 :!via `Reset`))
            (:`then_1`
              (`self.K2_SetActorRotation` (`KismetMathLibrary.RInterpTo` (`self.K2_GetActorRotation`) (`KismetMathLibrary.ComposeRotators` (`SplineComponent.GetRotationAtDistanceAlongSpline` (`/Game/TheLongWalk/BP_Chemin.CHemin` (`self.refchemin`)) (`self.distanceactuelle`) "World") (`self.TARGET ROTATION`)) (`GameplayStatics.GetWorldDeltaSeconds`) 5.0)))))))
    (:`then_1`
      (bind _returnvalue (`|CreateWidget` "/Game/TheLongWalk/WDG_Avancer.WDG_Avancer_C"))
      (`UserWidget.AddToViewport` _returnvalue 0)
      (set `PlayerController.bShowMouseCursor` true (`GameplayStatics.GetPlayerController` 0)))))

(event `self.ReceiveTick`
  (params (DeltaSeconds :type "Float (single-precision)"))
  ; Comment
  (`|ExecutionSequence`
    (:`then_0`
      (goto _label))
    (:`then_1`
      (if (`self.lAMPEALLUME`)
        (set `self.BATTERIE` (`KismetMathLibrary.FClamp` (* (- (`self.BATTERIE`) (`GameplayStatics.GetWorldDeltaSeconds`)) 0.01)))
        (if true
          _)))))

(event `Key|F`
  (params (Key :type "Key Structure"))
  ; Comment
  (:`Pressed`
    (`/Engine/EditorBlueprintResources/StandardMacros.FlipFlop` :!label _label_3
      (:`A`
        (`GameplayStatics.PlaySound2D` "/Engine/VREditor/Sounds/UI/Click_on_Button.Click_on_Button" 1.0 1.0 0.0 null null)
        (`LightComponent.SetIntensity` (`self.SpotLight`) 91055.71875)
        (set `self.lAMPEALLUME` true))
      (:`B`
        (`GameplayStatics.PlaySound2D` "/Engine/VREditor/Sounds/UI/Click_on_Button.Click_on_Button" 1.0 1.0 0.0 null null)
        (`LightComponent.SetIntensity` (`self.SpotLight`) 0.0)
        (set `self.lAMPEALLUME` false))))
  (:`Released`
    (goto _label_3)))

(fn `UserConstructionScript`)